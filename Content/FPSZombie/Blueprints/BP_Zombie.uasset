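; BP_Zombie is an FPS zombie enemy Blueprint that manages its overhead health bar widget.
; On BeginPlay it binds the widget to itself and refreshes HP, with UpdateHP and DisableHPBar events to refresh or hide it later.
; Each Tick it traces from above its mesh to the player camera on the Camera channel, showing the bar only when the trace hits the player character.
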(event EventBeginPlay
  (bind _asfpszombie_healthbar (Utilities|Casting|CastToFPSZombie_Healthbar (UserInterface|GetWidget (Variables|Default|GetHealthBar))))
  (Default|SetOwner _asfpszombie_healthbar self)
  (Default|UpdateHP _asfpszombie_healthbar))

(event Collision|EventActorBeginOverlap
  (params (OtherActor :type Actor%20Object%20Reference)))

(event EventTick
  (params (DeltaSeconds :type Float%20%28single-precision%29))
  (bind (_outhit _returnvalue) (Collision|LineTraceByChannel (+ (Transformation|GetWorldLocation (Variables|Character|GetMesh)) "0.000000,0.000000,160.000000") (Camera|GetCameraLocation (Game|GetPlayerCameraManager 0)) "TraceTypeQuery2" false 0 "None"))
  (if _returnvalue
    (Utilities|Casting|CastToFPSCharacterPlayer (.HitActor (Collision|BreakHitResult _outhit))
      (:then
        (Widget|SetVisibility (UserInterface|GetWidget (Variables|Default|GetHealthBar)) "Visible"))
      (:CastFailed
        (Widget|SetVisibility (UserInterface|GetWidget (Variables|Default|GetHealthBar)) "Hidden" :!label _label)))
    (else
      (goto _label))))

(event EventUpdateHP
  (bind _healthbar (Variables|Default|GetHealthBar))
  (Utilities|IsValid _healthbar
    (:Is%20Valid
      (bind _asfpszombie_healthbar (Utilities|Casting|CastToFPSZombie_Healthbar (UserInterface|GetWidget _healthbar)))
      (Default|UpdateHP _asfpszombie_healthbar))))

(event EventDisableHPBar
  (Development|SetHiddeninGame (Variables|Default|GetHealthBar) true true))

(fn ConstructionScript)