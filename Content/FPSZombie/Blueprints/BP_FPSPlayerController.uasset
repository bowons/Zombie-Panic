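; Player controller for the FPS zombie game that owns the crosshair HUD and plays camera shakes.
; It creates the crosshair widget on BeginPlay and updates it from the player's selected weapon on ChangeWeapon.
; Each tick it hides the crosshair while the player is aiming, swapping or reloading.
; Two events play the same world camera shake at the pawn's location, with a tighter radius for firing.
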(event EventBeginPlay
  (bind _returnvalue (UserInterface|CreateWidget "/Game/FPSZombie/Widget/FPSZombie_Crosshair.FPSZombie_Crosshair_C"))
  (bind _output_get (Variables|Default|SetCrossHairHUD _returnvalue))
  (UserInterface|Viewport|AddtoViewport _output_get 0))

(event EventTick
  (params (DeltaSeconds :type Float%20%28single-precision%29))
  (bind _crosshairhud (Variables|Default|GetCrossHairHUD))
  (bind _asfpscharacter_player (Utilities|Casting|CastToFPSCharacterPlayer (Game|Player|GetPlayerPawn 0)))
  (Utilities|IsValid _asfpscharacter_player
    (:Is%20Valid
      (if (CallFunction|IsActing _asfpscharacter_player)
        (Widget|SetVisibility _crosshairhud "Hidden")
        (else
          (Widget|SetVisibility _crosshairhud "Visible"))))))

(event EventChangeWeapon
  (bind _asfpscharacter_player (Utilities|Casting|CastToFPSCharacterPlayer (Game|Player|GetPlayerPawn 0)))
  (Utilities|IsValid (Variables|/Script/FPSZombie.FPSCharacterPlayer|GetSelectedWeapon _asfpscharacter_player)
    (:Is%20Valid
      (Default|UpdateCrossHair (Variables|Default|GetCrossHairHUD) (Variables|/Script/FPSZombie.FPSCharacterPlayer|GetSelectedWeapon _asfpscharacter_player)))))

(event EventShakeCamera
  (Camera|PlayWorldCameraShake "/Game/FPSZombie/Blueprints/BP_PlayerCamshake.BP_PlayerCamshake_C" (Transformation|GetActorLocation (Game|Player|GetPlayerPawn 0)) 3.5e+02 3.5e+02))

(event EventFiringCamShake
  (Camera|PlayWorldCameraShake "/Game/FPSZombie/Blueprints/BP_PlayerCamshake.BP_PlayerCamshake_C" (Transformation|GetActorLocation (Game|Player|GetPlayerPawn 0)) 5e+01 8e+01))

(fn ConstructionScript)

(fn IsActing
  (params (Player :type FPS%20Character%20Player%20Object%20Reference))
  (return (Math|Boolean|ORBoolean (Variables|/Script/FPSZombie.FPSCharacterPlayer|GetbIsAiming Player) (Variables|/Script/FPSZombie.FPSCharacterPlayer|GetbIsSwaping Player) (Variables|/Script/FPSZombie.FPSWeaponBase|GetbIsReloading (Variables|/Script/FPSZombie.FPSCharacterPlayer|GetSelectedWeapon Player)))))